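; BP_Lib00 is a geometry Blueprint, apparently a "Lib" building piece, with two configurable floor inserts.
; Its construction script adds two static mesh components at the relative locations of LibInsertFloor0 and LibInsertFloor1.
; The Insert0 and Insert1 indices each select that component's mesh from the InsertFloors array.
; It has no active runtime logic, as the event graph holds only disabled default nodes.
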(event EventBeginPlay)

(event Collision|EventActorBeginOverlap
  (params (OtherActor :type Actor%20Object%20Reference)))

(event EventTick
  (params (DeltaSeconds :type Float%20%28single-precision%29)))

(fn ConstructionScript
  (bind _returnvalue (AddComponent|AddStaticMeshComponent false))
  (Transformation|SetRelativeLocation _returnvalue (Variables|/Script/Engine.SceneComponent|GetRelativeLocation (Variables|Default|GetLibInsertFloor_0)) false false)
  (Components|StaticMesh|SetStaticMesh _returnvalue (Utilities|Array|Get(acopy) (Variables|Default|GetInsertFloors) (Variables|Default|GetInsert0)))
  (bind _returnvalue_2 (AddComponent|AddStaticMeshComponent false))
  (Transformation|SetRelativeLocation _returnvalue_2 (Variables|/Script/Engine.SceneComponent|GetRelativeLocation (Variables|Default|GetLibInsertFloor_1)) false false)
  (Components|StaticMesh|SetStaticMesh _returnvalue_2 (Utilities|Array|Get(acopy) (Variables|Default|GetInsertFloors) (Variables|Default|GetInsert1))))