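; BP_ringPLacement is a construction-time placement actor that arranges copies of a chosen mesh in a ring or arc.
; Its construction script assigns Mesh to an InstancedStaticMesh component, then adds NumItems instances at radius Dist in the local XY plane, stepped by Angle degrees.
; Each instance is yawed to match its angle, so its X axis points along the radius.
; The event graph holds no active logic.
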(event EventBeginPlay)

(event Collision|EventActorBeginOverlap
  (params (OtherActor :type Actor%20Object%20Reference)))

(event EventTick
  (params (DeltaSeconds :type Float%20%28single-precision%29)))

(fn ConstructionScript
  (Components|StaticMesh|SetStaticMesh (Variables|Default|GetInstancedStaticMesh) (Variables|Default|GetMesh))
  (for _index (range 0 (- (Variables|Default|GetNumItems) 1))
    (Components|InstancedStaticMesh|AddInstance (Variables|Default|GetInstancedStaticMesh) (Math|Transform|MakeTransform (* (Math|Vector|MakeVector (Math|Trig|Cos(Degrees) (* _index (Variables|Default|GetAngle))) (Math|Trig|Sin(Degrees) (* _index (Variables|Default|GetAngle))) 0.0) (Variables|Default|GetDist)) (Math|Rotator|MakeRotator 0.0 0.0 (* _index (Variables|Default|GetAngle)))))))